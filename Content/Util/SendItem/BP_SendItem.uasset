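; BP_SendItem is an actor that delivers a stored item stack to a target inventory, optionally shown as an item flying along an arc.
; Fire either waits out a delay invisibly or spawns a BP_CostEffectActor, whose target Tick keeps updated.
; Arrival or destruction triggers one guarded completion, so interrupted sends still deliver.
; Only authority runs Deliver, returning leftovers to the source inventory, then dropping any remainder at the target.
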(event `On Destroyed` :!signature `self.OnDestroyed`
  (params (DestroyedActor :type "Actor Object Reference"))
  (if (not (`self.Finished`)) :!label _label
    (set `self.Finished` true)
    (`self.Done` self)
    (if (`self.ToPlayer`)
      (`GameplayStatics.PlaySoundAtLocation` "/PowerSuit/Assets/Audio/Item_PickUp_Cue.Item_PickUp_Cue" (`self.K2_GetActorLocation` self) (struct) 0.5 1.0 0.0 "/PowerSuit/Assets/Audio/PickUpItem_Attenuation.PickUpItem_Attenuation" null null))
    (`/Engine/EditorBlueprintResources/ActorMacros.Switch Has Authority`
      (:`Authority`
        (`self.Deliver`))
      (:`Remote`
        (`self.K2_DestroyActor`)))))

(event `Fire owning Client`
  (params (DisableTrailParticles :type Boolean))
  (`self.SpawnAndAttach` DisableTrailParticles))

(event `On Reached Target`
  (goto _label))

(event `Fire`
  (params (`Disable Trail Particles` :type Boolean) (`No Visuals Delivery` :type Boolean) (`Delay before Sending` :type "Float (double-precision)"))
  (bind _flyactor (`self.FlyActor`))
  (set `self.Instant` `No Visuals Delivery`)
  (set `self.Delay` `Delay before Sending`)
  (set `self.Started` (`KismetMathLibrary.Now`))
  (if (`self.Instant`)
    ;[1 1 1] Instant actors don't have any visuals, they just wait the time and then deliver
    (`KismetSystemLibrary.Delay` `Delay before Sending`)
    (goto _label)
    (else
      (`self.Fire owning Client` `Disable Trail Particles`)
      (add `/Game/FactoryGame/Buildable/Factory/-Shared/BP_CostEffectActor.OnReachedTarget` _flyactor (delegate `On Reached Target`))
      (add `self.OnDestroyed` _flyactor (delegate `On Destroyed`)))))

(event `self.ReceiveTick`
  (params (DeltaSeconds :type "Float (single-precision)"))
  (`/Engine/EditorBlueprintResources/StandardMacros.IsValid` (`self.FlyActor`)
    (:`Is Valid`
      (set `/Game/FactoryGame/Buildable/Factory/-Shared/BP_CostEffectActor.mTargetLocation` (`self.K2_GetActorLocation` (`self.Target Actor for Location`)) (`self.FlyActor`)))
    (:`Is Not Valid`
      (if (`self.Finished`)
        (`self.K2_DestroyActor`)
        (else
          (`KismetSystemLibrary.Delay` 0.2)
          (`self.On Reached Target`))))))

(fn `Deliver`
  (bind _stored_stack (`self.Stored Stack`))
  (bind (_out_numitems _out_item) (`FGInventoryLibrary.BreakInventoryStack` (`self.Stored Stack`)))
  (bind (_out_numitems_2 _out_item_2) (`FGInventoryLibrary.BreakInventoryStack` _stored_stack))
  (bind _returnvalue (`FGInventoryComponent.AddStack` (`self.Target Inventory`) _stored_stack false))
  (bind _returnvalue_2 (- _out_numitems_2 _returnvalue))
  (if (> _returnvalue_2 0)
    (`BlueprintLoggingLibrary.LogError` (`KismetStringLibrary.Concat_StrStr` "Send Item Partially Failed ! Placing " (`KismetStringLibrary.Conv_IntToString` _returnvalue_2) "Back to Inventory : " (`KismetSystemLibrary.GetPathName` (`self.Source Inventory`))))
    (bind _returnvalue_3 (`FGInventoryComponent.AddStack` (`self.Source Inventory`) (`FGInventoryLibrary.MakeInventoryStack` _returnvalue_2 _out_item_2) false))
    (bind _returnvalue_4 (- _returnvalue_2 _returnvalue_3))
    (if (> _returnvalue_4 0)
      (`BlueprintLoggingLibrary.LogError` (`KismetStringLibrary.Concat_StrStr` "Send Item also failed to Place back to Source Inventory! Placing " (`KismetStringLibrary.Conv_IntToString` _returnvalue_4) " Item : " (`KismetSystemLibrary.GetClassDisplayName` (`FGInventoryLibrary.BreakInventoryItem` _out_item_2)) " on the Ground by Target"))
      (`FGItemPickup_Spawnable.CreateItemDrop` (`self.Target Inventory`) (`FGInventoryLibrary.MakeInventoryStack` _returnvalue_4 _out_item_2) (`self.K2_GetActorLocation` (`ActorComponent.GetOwner` (`self.Target Inventory`))) (struct) "/Game/FactoryGame/Resource/BP_ItemPickup_Spawnable.BP_ItemPickup_Spawnable_C"))
    (else
      (`BlueprintLoggingLibrary.LogVerbose` (`KismetStringLibrary.Concat_StrStr` "Completed item delivery of " (`KismetStringLibrary.Conv_IntToString` _out_numitems) " x " (`KismetSystemLibrary.GetClassDisplayName` (`FGInventoryLibrary.BreakInventoryItem` _out_item))))))
  (`self.K2_DestroyActor`))

(fn `UserConstructionScript`)