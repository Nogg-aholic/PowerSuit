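; BP_Attachment_Cheat is a debug power suit attachment with directly settable condition, trigger and consumption values.
; Server set-value events use an index to write the bool and float variables, which the condition and power/fuel consumption getters return without scaling by delta time.
; Lifecycle events, setters and stat receipt log through LogError, with begin play, install and destroy split by network authority.
; Tick events are empty.
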(event `self.ReceiveBeginPlay`
  (`/Engine/EditorBlueprintResources/ActorMacros.Switch Has Authority`
    (:`Authority`
      (`BlueprintLoggingLibrary.LogError` "Attachment Begin Play Server"))
    (:`Remote`
      (`BlueprintLoggingLibrary.LogError` "Attachment Begin Play Remote"))))

(event `self.ReceiveDestroyed`
  (`/Engine/EditorBlueprintResources/ActorMacros.Switch Has Authority`
    (:`Authority`
      (`BlueprintLoggingLibrary.LogError` "Attachment Destroyed Server"))
    (:`Remote`
      (`BlueprintLoggingLibrary.LogError` "Attachment Destroyed Remote"))))

(event `self.AttachmentInstalled`
  (params (Item :type "InventoryItem Structure"))
  (`/Engine/EditorBlueprintResources/ActorMacros.Switch Has Authority`
    (:`Authority`
      (`BlueprintLoggingLibrary.LogError` "Attachment Installed Server"))
    (:`Remote`
      (`BlueprintLoggingLibrary.LogError` "Attachment Installed Remote"))))

(event `self.AttachmentUnInstalled`
  (`BlueprintLoggingLibrary.LogError` "Attachment Un-Installed"))

(event `self.AttachmentPreTick`
  (params (DeltaTime :type "Float (single-precision)")))

(event `self.AttachmentTick`
  (params (DeltaTime :type "Float (single-precision)")))

(event `self.AttachmentPostTick`
  (params (DeltaTime :type "Float (single-precision)")))

(event `self.ServerSetBoolValue`
  (params (Value :type Boolean) (Index :type Byte))
  (if (== Index 0)
    (set `self.ConditionMet` Value)
    (`BlueprintLoggingLibrary.LogError` "Server BP Set Bool")
    (else
      (set `self.ShouldTriggerActive` Value)
      (`BlueprintLoggingLibrary.LogError` "Remote  BP Set Bool"))))

(event `self.ServerSetFloatValue`
  (params (Value :type "Float (single-precision)") (Index :type Byte))
  (if (== Index 0)
    (set `self.PowerConsumption` Value)
    (`BlueprintLoggingLibrary.LogError` "Server BP Set Float")
    (else
      (set `self.FuelConsumption` Value)
      (`BlueprintLoggingLibrary.LogError` "Remote  BP Set Float"))))

(fn `GetDeltaFuelConsumption`
  (params (DeltaTime :type "Float (double-precision)"))
  (returns (ReturnValue :type "Float (double-precision)"))
  (return (`self.FuelConsumption`)))

(fn `GetDeltaPowerConsumption`
  (params (DeltaTime :type "Float (double-precision)"))
  (returns (ReturnValue :type "Float (double-precision)"))
  (return (`self.PowerConsumption`)))

(fn `GetIsConditionMet`
  (returns (ReturnValue :type Boolean))
  (return (`self.ConditionMet`)))

(fn `RecieveModuleStats`
  (params (DefaultStats :type "EquipmentStats Structure"))
  (returns (ReturnValue :type "EquipmentStats Structure"))
  (`BlueprintLoggingLibrary.LogError` "Recieve Stats Installed")
  (return (`self.AttachmentStats`)))

(fn `ShouldSave`
  (returns (ReturnValue :type Boolean))
  (return true))

(fn `UserConstructionScript`)