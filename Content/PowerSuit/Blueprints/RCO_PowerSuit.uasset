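; Remote call object for the power suit that passes player movement state and input to the server copy of the suit.
; Paired Remote and Server events forward each value, such as movement modes, sprint, slide, hover, hotkey acceleration, axes and pipe velocity, then write it onto the passed-in suit object.
; Up and down acceleration changes also reset vertical velocity, and many setters log through LogError, apparently for debugging.
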(event `Remote_EMovementMode`
  (params (InputPin :type "/Game/PowerSuit/Equipment/PowerSuit/Equip_PowerSuit_Parent Object Reference") (Enumerator :type Byte))
  (`self.Server_EMovementMode` InputPin Enumerator))

(event `Server_EMovementMode`
  (params (InputPin :type "/Game/PowerSuit/Equipment/PowerSuit/Equip_PowerSuit_Parent Object Reference") (Enumerator :type Byte))
  (set `PowerSuit.nMovementMode` (cast `EMovementMode` Enumerator) InputPin))

(event `Remote_EMovementModeCustom`
  (params (InputPin :type "/Game/PowerSuit/Equipment/PowerSuit/Equip_PowerSuit_Parent Object Reference") (Enumerator :type Byte))
  (`self.Server_EMovementModeCustom` InputPin Enumerator))

(event `Server_EMovementModeCustom`
  (params (InputPin :type "/Game/PowerSuit/Equipment/PowerSuit/Equip_PowerSuit_Parent Object Reference") (Enumerator :type Byte))
  (set `PowerSuit.nCustomMovementMode` Enumerator InputPin))

(event `Remote_PiepeVel`
  (params (InputPin :type "/Game/PowerSuit/Equipment/PowerSuit/Equip_PowerSuit_Parent Object Reference") (Sppeed :type "Float (double-precision)"))
  (`self.Server_PiepeVel` InputPin Sppeed))

(event `Server_PiepeVel`
  (params (InputPin :type "/Game/PowerSuit/Equipment/PowerSuit/Equip_PowerSuit_Parent Object Reference") (Speed :type "Float (double-precision)"))
  (bind _output_get (set `PowerSuit.nPipeVelocity` Speed InputPin))
  (`SMLBlueprintLibrary.LogError` (`KismetStringLibrary.Conv_DoubleToString` _output_get)))

(event `Server_IsSprinting`
  (params (mIsSprinting :type Boolean) (InputPin :type "/Game/PowerSuit/Equipment/PowerSuit/Equip_PowerSuit_Parent Object Reference"))
  (bind _output_get (set `PowerSuit.nIsSprinting` mIsSprinting InputPin))
  (`SMLBlueprintLibrary.LogError` "Server_IsSprinting")
  (`SMLBlueprintLibrary.LogError` (`KismetStringLibrary.Conv_BoolToString` _output_get)))

(event `Remote_IsSprinting`
  (params (mIsSprinting :type Boolean) (InputPin :type "/Game/PowerSuit/Equipment/PowerSuit/Equip_PowerSuit_Parent Object Reference"))
  (`self.Server_IsSprinting` mIsSprinting InputPin))

(event `Server_IsSliding`
  (params (mIsSliding :type Boolean) (InputPin :type "/Game/PowerSuit/Equipment/PowerSuit/Equip_PowerSuit_Parent Object Reference"))
  (bind _output_get (set `PowerSuit.nIsSliding` mIsSliding InputPin))
  (`SMLBlueprintLibrary.LogError` "Server_IsSliding")
  (`SMLBlueprintLibrary.LogError` (`KismetStringLibrary.Conv_BoolToString` _output_get)))

(event `Remote_IsSliding`
  (params (mIsSliding :type Boolean) (InputPin :type "/Game/PowerSuit/Equipment/PowerSuit/Equip_PowerSuit_Parent Object Reference"))
  (`self.Server_IsSliding` mIsSliding InputPin))

(event `Server_HotKeyDirectionalAcceleration`
  (params (HotKeyDirectionalAcceleration :type Boolean) (InputPin :type "/Game/PowerSuit/Equipment/PowerSuit/Equip_PowerSuit_Parent Object Reference"))
  (bind _output_get (set `PowerSuit.HotKeyDirectionalAccelration` HotKeyDirectionalAcceleration InputPin))
  (`SMLBlueprintLibrary.LogError` "Server_HotKeyDirectionalAcceleration")
  (`SMLBlueprintLibrary.LogError` (`KismetStringLibrary.Conv_BoolToString` _output_get)))

(event `Remote_HotKeyDirectionalAcceleration`
  (params (HotKeyDirectionalAcceleration :type Boolean) (InputPin :type "/Game/PowerSuit/Equipment/PowerSuit/Equip_PowerSuit_Parent Object Reference"))
  (`self.Server_HotKeyDirectionalAcceleration` HotKeyDirectionalAcceleration InputPin))

(event `Server_HotKeyDownAccel`
  (params (`HotKeyDown Accel` :type Boolean) (InputPin :type "/Game/PowerSuit/Equipment/PowerSuit/Equip_PowerSuit_Parent Object Reference"))
  (bind _output_get (set `PowerSuit.HotKeyDownAccelration` `HotKeyDown Accel` InputPin))
  (`SMLBlueprintLibrary.LogError` "Server_HotKeyDownAccel")
  (`SMLBlueprintLibrary.LogError` (`KismetStringLibrary.Conv_BoolToString` _output_get))
  (`/Game/PowerSuit/Equipment/PowerSuit/Equip_PowerSuit_Parent.ResetVerticalVelocity` InputPin))

(event `Remote_HotKeyDownAccel`
  (params (HotKeyDown :type Boolean) (InputPin :type "/Game/PowerSuit/Equipment/PowerSuit/Equip_PowerSuit_Parent Object Reference"))
  (`self.Server_HotKeyDownAccel` HotKeyDown InputPin))

(event `Server_HotKeyUpAccel`
  (params (`HotKeyUp Accell` :type Boolean) (InputPin :type "/Game/PowerSuit/Equipment/PowerSuit/Equip_PowerSuit_Parent Object Reference"))
  (bind _output_get (set `PowerSuit.HotKeyUpAccelration` `HotKeyUp Accell` InputPin))
  (`SMLBlueprintLibrary.LogError` "Server_HotKeyUpAccel")
  (`SMLBlueprintLibrary.LogError` (`KismetStringLibrary.Conv_BoolToString` _output_get))
  (`/Game/PowerSuit/Equipment/PowerSuit/Equip_PowerSuit_Parent.ResetVerticalVelocity` InputPin))

(event `Remote_HotKeyUpAccel`
  (params (HotKeyUp :type Boolean) (InputPin :type "/Game/PowerSuit/Equipment/PowerSuit/Equip_PowerSuit_Parent Object Reference"))
  (`self.Server_HotKeyUpAccel` HotKeyUp InputPin))

(event `Server_Hovering`
  (params (`Hovering ` :type Boolean) (InputPin :type "/Game/PowerSuit/Equipment/PowerSuit/Equip_PowerSuit_Parent Object Reference"))
  (bind _output_get (set `PowerSuit.Hovering` `Hovering ` InputPin))
  (`SMLBlueprintLibrary.LogError` "Server_Hovering")
  (`SMLBlueprintLibrary.LogError` (`KismetStringLibrary.Conv_BoolToString` _output_get)))

(event `Remote_Hovering`
  (params (`Hovering ` :type Boolean) (InputPin :type "/Game/PowerSuit/Equipment/PowerSuit/Equip_PowerSuit_Parent Object Reference"))
  (`self.Server_Hovering` `Hovering ` InputPin))

(event `Server_ISRemote`
  (params (`is Remote` :type Boolean) (InputPin :type "/Game/PowerSuit/Equipment/PowerSuit/Equip_PowerSuit_Parent Object Reference"))
  (bind _output_get (set `PowerSuit.nRemoteControlled` `is Remote` InputPin))
  (`SMLBlueprintLibrary.LogError` "Server_ISRemote")
  (`SMLBlueprintLibrary.LogError` (`KismetStringLibrary.Conv_BoolToString` _output_get)))

(event `Remote_ISRemote`
  (params (`is Remote` :type Boolean) (InputPin :type "/Game/PowerSuit/Equipment/PowerSuit/Equip_PowerSuit_Parent Object Reference"))
  (`self.Server_ISRemote` `is Remote` InputPin))

(event `Server_XAxis`
  (params (Xaxis :type "Float (double-precision)") (InputPin :type "/Game/PowerSuit/Equipment/PowerSuit/Equip_PowerSuit_Parent Object Reference"))
  (set `PowerSuit.Xaxis` Xaxis InputPin))

(event `Remote_XAxis`
  (params (Xaxis :type "Float (double-precision)") (InputPin :type "/Game/PowerSuit/Equipment/PowerSuit/Equip_PowerSuit_Parent Object Reference"))
  (`self.Server_XAxis` Xaxis InputPin))

(event `Server_YAxis`
  (params (Yaxis :type "Float (double-precision)") (InputPin :type "/Game/PowerSuit/Equipment/PowerSuit/Equip_PowerSuit_Parent Object Reference"))
  (set `PowerSuit.Yaxis` Yaxis InputPin))

(event `Remote_YAxis`
  (params (Yaxis :type "Float (double-precision)") (InputPin :type "/Game/PowerSuit/Equipment/PowerSuit/Equip_PowerSuit_Parent Object Reference"))
  (`self.Server_YAxis` Yaxis InputPin))

(event `RepVector_Server`
  (params (ReplicatedVector :type "Vector Structure") (InputPin :type "/Game/PowerSuit/Equipment/PowerSuit/Equip_PowerSuit_Parent Object Reference"))
  (set `/Game/PowerSuit/Equipment/PowerSuit/Equip_PowerSuit_Parent.ReplicatedVector` ReplicatedVector InputPin))

(event `RepVector_Remote`
  (params (ReplicatedVector :type "Vector Structure") (InputPin :type "/Game/PowerSuit/Equipment/PowerSuit/Equip_PowerSuit_Parent Object Reference"))
  (`self.RepVector_Server` ReplicatedVector InputPin))

(fn `NewFunction_0`
  (params (IDX :type Integer) (Obj :type "Object Object Reference")))